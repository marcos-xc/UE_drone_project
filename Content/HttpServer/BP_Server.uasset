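; Camera actor that runs HTTP servers for remote control of a scene-capture camera and a BP_drone, saving images to Saved/Python.
; PUT requests carry JSON that drives timeline-based, range-limited rotation and FOV changes, capturing frames as they finish.
; A Reset field applies drone flight settings, restores the camera and restarts the servers.
; A second-port GET route, like the PUT reply, returns camera and drone state as JSON.
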(event Custom|Port1Event
  (params (HttpRequest :type Blueprint%20Http%20Request%20Structure%20%28by%20ref%29) (HttpResponse :type Blueprint%20Http%20Response%20Structure))
  (Utilities|FlowControl|Sequence
    (:then_0
      (Variables|Default|SetCameraDone true)
      (Utilities|MResponse HttpResponse))
    (:then_1
      (|New (Class|BlueprintHttpServerLibrary|GetBody HttpRequest)))))

(event Custom|Event_FOV
  (bind _fov (Variables|Default|GetFOV))
  (if (Audio|Components|Audio|IsPlaying _fov)
    (CallFunction|CapturePython))
  (Components|Timeline|PlayfromStart _fov))

(event Custom|CaptureButton
  (bind _returnvalue (Class|BlueprintPathsLibrary|ProjectSavedDir))
  ;[1 0.4115 0.4115] 存照片
  (Development|PrintString _returnvalue)
  (Class|SavePhotoPawn|SaveImage (Utilities|String|Append _returnvalue "Button/") (Utilities|String|Append "Drone_" (Utilities|String|ToString(Integer) (Variables|/Game/HttpServer/BP_drone.BP_drone_C|GetWRJNum (Variables|Default|GetBP_Drone)))) false true))

(event Custom|HttpInit
  (Utilities|IsValid (Variables|Default|GetHTTP%20Server)
    (:Is%20Valid
      (Class|BlueprintHttpServer|Stop (Variables|Default|GetHTTP%20Server))
      (Variables|Default|SetHTTP%20Server 0)
      (Class|BlueprintHttpServer|Stop (Variables|Default|GetHTTP%20Server_0))
      (Variables|Default|SetHTTP%20Server_0 0))
    (:Is%20Not%20Valid
      _))
  (Utilities|FlowControl|Sequence
    (:then_0
      (Variables|Default|SetHTTP%20Server (Class|BlueprintHttpServer|CreateHttpServer))
      (Class|BlueprintHttpServerLibrary|AddRoute (Variables|Default|GetHTTP%20Server) "Put" (Variables|Default|GetRoute) true (delegate Custom|Port1Event))
      (|Listen (Variables|Default|GetHTTP%20Server) (Variables|Default|GetIP) (Variables|Default|GetPort)
        (:OnListening
          (Development|PrintString "Listen"))
        (:OnFailed
          (Development|PrintString "Faild"))))
    (:then_1
      (|Port2))))

(event Custom|Event_Rotation
  (params (XorZ :type String) (MoveValue :type Float%20%28double-precision%29))
  (bind _rotate (Variables|Default|GetRotate))
  (Variables|Default|SetYorZ XorZ)
  (Variables|Default|SetMoveValue MoveValue)
  (Variables|Default|SetNew%20Relative%20Rotation (CallFunction|FRotation))
  (if (Audio|Components|Audio|IsPlaying _rotate)
    (CallFunction|CapturePython))
  (Components|Timeline|PlayfromStart _rotate))

(event Custom|Init
  (params (IP :type String) (Port :type Integer))
  (Utilities|IsValid (Variables|Default|GetHTTP%20Server)
    (:Is%20Valid
      (Class|BlueprintHttpServer|Stop (Variables|Default|GetHTTP%20Server))
      (Variables|Default|SetHTTP%20Server 0)
      (Variables|Default|SetPort Port)
      (Variables|Default|SetIP IP)
      (Variables|Default|SetHTTP%20Server (Class|BlueprintHttpServer|CreateHttpServer))
      (Class|BlueprintHttpServerLibrary|AddRoute (Variables|Default|GetHTTP%20Server) "Put" (Variables|Default|GetRoute) true (delegate Custom|Port1Event))
      (|Listen (Variables|Default|GetHTTP%20Server) (Variables|Default|GetIP) (Variables|Default|GetPort)
        (:OnListening
          (Development|PrintString "Listen"))
        (:OnFailed
          (Development|PrintString "Faild"))))))

(event Custom|Event_Roatation_Web
  (bind _rotate (Variables|Default|GetRotate))
  (Variables|Default|SetNew%20Relative%20Rotation (CallFunction|FRotation))
  (if (Audio|Components|Audio|IsPlaying _rotate)
    (CallFunction|CapturePython))
  (Components|Timeline|PlayfromStart _rotate))

(event Custom|CapturePython
  ;[1 0.4115 0.4115] 存照片
  (Class|SavePhotoPawn|SaveImage (Utilities|String|Append (Class|BlueprintPathsLibrary|ProjectSavedDir) "Python/") (Utilities|String|Append "Capture_" (Utilities|String|ToString(Integer) (Math|Integer|%(Integer) (Variables|Default|GetCaptureInt_Web) 10))) true true))

(event Custom|CustomEvent_0
  (params (Actor :type Actor%20Object%20Reference) (EndPlayReason :type EEndPlayReason%20Enum :default "Destroyed"))
  (Development|PrintString "End")
  (Class|BlueprintHttpServer|Stop (Variables|Default|GetHTTP%20Server))
  (Class|BlueprintHttpServer|Stop (Variables|Default|GetHTTP%20Server_0)))

(event Custom|CapturePython_UI
  ;[1 0.4115 0.4115] 存照片
  (Class|SavePhotoPawn|SaveImage (Utilities|String|Append (Class|BlueprintPathsLibrary|ProjectSavedDir) "Python/") "Capture" true true))

(event Custom|InitTrans
  ;[1 0.436 0] 初始化信息
  (Audio|Components|Audio|Stop (Variables|Default|GetRotate))
  (Transformation|SetActorTransform (Variables|Default|GetActorInitTransform))
  (Audio|Components|Audio|Stop (Variables|Default|GetFOV))
  (Camera|SetFieldOfView (Variables|Default|GetCamera) 9e+01))

(event Custom|SetCameraHeight
  (params (Height :type Float%20%28double-precision%29))
  (bind _returnvalue (Transformation|GetActorLocation))
  (Transformation|SetActorLocation (Math|Vector|MakeVector (.x _returnvalue) (.y _returnvalue) Height) false false))

(event EventBeginPlay
  (bind _outactors (Actor|GetAllActorsOfClass "/Game/HttpServer/BP_drone.BP_drone_C"))
  (Variables|Default|SetBP_Drone (Utilities|Array|Get(acopy) _outactors))
  (Variables|Default|SetActorInitTransform (Transformation|GetActorTransform))
  (Variables|/Script/Engine.PlayerController|SetbShowMouseCursor (Game|GetPlayerController 0) true)
  (Utilities|FlowControl|Sequence
    (:then_0
      (Utilities|IsValid (Variables|Default|GetHTTP%20Server)
        (:Is%20Valid
          (Class|BlueprintHttpServer|Stop (Variables|Default|GetHTTP%20Server))
          (Variables|Default|SetHTTP%20Server 0)
          (Class|BlueprintHttpServer|Stop (Variables|Default|GetHTTP%20Server_0))
          (Variables|Default|SetHTTP%20Server_0 0))
        (:Is%20Not%20Valid
          _))
      (Utilities|FlowControl|Sequence
        (:then_0
          (Variables|Default|SetHTTP%20Server (Class|BlueprintHttpServer|CreateHttpServer))
          (Class|BlueprintHttpServerLibrary|AddRoute (Variables|Default|GetHTTP%20Server) "Put" (Variables|Default|GetRoute) true (delegate Custom|Port1Event))
          (|Listen (Variables|Default|GetHTTP%20Server) (Variables|Default|GetIP) (Variables|Default|GetPort)
            (:OnListening
              (Development|PrintString "Listen"))
            (:OnFailed
              (Development|PrintString "Faild"))))
        (:then_1
          (|Port2))))
    (:then_1
      (Game|BindEventtoOnEndPlay (delegate Custom|CustomEvent_0)))
    (:then_2
      ;[0.474 0 0] 无人机飞行
      (bind _outactors_2 (Actor|GetAllActorsOfClass "/Game/HttpServer/BP_drone.BP_drone_C"))
      (for _array_element _outactors_2
        (Default|EventFly _array_element)))))

(event Collision|EventActorBeginOverlap
  (params (OtherActor :type Actor%20Object%20Reference)))

(event EventTick
  (params (DeltaSeconds :type Float%20%28single-precision%29)))

(event Input|KeyboardEvents|2
  (params (Key :type Key%20Structure :default "None"))
  (:Pressed
    (for _index (range 0 (Math|Random|RandomIntegerinRange 3 7))
      (Development|PrintString (Utilities|String|ToString(Integer) _index)))))

(fn ConstructionScript)

(fn FRotation
  (bind _returnvalue (Transformation|GetActorRotation))
  (bind _returnvalue_2 (Transformation|GetActorRotation))
  (bind _movevalue (Variables|Default|GetMoveValue))
  (bind _movevalue_2 (Variables|Default|GetMoveValue))
  (bind (_roll _pitch _yaw) (Math|Rotator|BreakRotator _returnvalue_2))
  (bind (_roll_2 _pitch_2 _yaw_2) (Math|Rotator|BreakRotator _returnvalue))
  (bind _returnvalue_3 (+ _pitch _movevalue_2))
  (bind _returnvalue_4 (+ _yaw_2 _movevalue))
  (switch string (Variables|Default|GetYorZ)
    (:Z
      (if (and (< _returnvalue_3 45.0) (> _returnvalue_3 -45.0))
        (return (Math|Rotator|MakeRotator _roll _returnvalue_3 _yaw))))
    (:Y
      (if (and (< _returnvalue_4 45.0) (> _returnvalue_4 -45.0))
        (return (Math|Rotator|MakeRotator _roll_2 _pitch_2 _returnvalue_4))))))

(event Custom|CustomEvent
  (params (HttpRequest :type Blueprint%20Http%20Request%20Structure%20%28by%20ref%29) (HttpResponse :type Blueprint%20Http%20Response%20Structure))
  (Utilities|MResponse HttpResponse))